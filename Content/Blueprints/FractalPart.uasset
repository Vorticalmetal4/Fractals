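; FractalPart is an actor that extends a chain of copies of itself as the player pawn overlaps each one.
; The first player overlap sets a one-time flag and spawns another FractalPart, offset by Separation with the same scale and zero rotation.
; It then calls SetRotations on the new part, which randomizes each HierarchicalInstancedStaticMesh instance's rotation on all axes while keeping location and scale.
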(event `self.ReceiveActorBeginOverlap`
  (params (OtherActor :type "Actor Object Reference"))
  (if (== OtherActor (`GameplayStatics.GetPlayerPawn` 0))
    (if (not (`self.wasActivated`))
      (set `self.wasActivated` true)
      (bind _returnvalue (`|SpawnActorFromClass` "FractalPart_C" (`KismetMathLibrary.MakeTransform` (+ (`self.K2_GetActorLocation`) (`self.Separation`)) (struct) (`self.GetActorScale3D`)) "Undefined" "OverrideRootScale" null null))
      (`self.SetRotations` _returnvalue))))

(fn `SetRotations`
  (bind _hierarchicalinstancedstaticmesh (`self.HierarchicalInstancedStaticMesh`))
  (for _index (range (+ (`InstancedStaticMeshComponent.GetInstanceCount` _hierarchicalinstancedstaticmesh) 1))
    (`InstancedStaticMeshComponent.UpdateInstanceTransform` _hierarchicalinstancedstaticmesh _index (`KismetMathLibrary.MakeTransform` (.location (`InstancedStaticMeshComponent.GetInstanceTransform` _hierarchicalinstancedstaticmesh _index false)) (`KismetMathLibrary.MakeRotator` (`KismetMathLibrary.Conv_IntToDouble` (`KismetMathLibrary.RandomIntegerInRange` 0 364)) (`KismetMathLibrary.Conv_IntToDouble` (`KismetMathLibrary.RandomIntegerInRange` 0 364)) (`KismetMathLibrary.Conv_IntToDouble` (`KismetMathLibrary.RandomIntegerInRange` 0 364))) (.scale (`InstancedStaticMeshComponent.GetInstanceTransform` _hierarchicalinstancedstaticmesh _index false))) false false false)))

(fn `UserConstructionScript`)